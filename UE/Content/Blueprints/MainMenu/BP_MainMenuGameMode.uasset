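; Main menu game mode that keeps Kronos matchmaking in step with changes in party connection.
; On BeginPlay it binds handlers to the connected-to-party and disconnected-from-party events.
; Both handlers cancel Kronos matchmaking if a search is running, so joining or leaving a party ends any active matchmaking.
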(event `self.ReceiveBeginPlay`
  ;[0 0 0] Cancel matchmaking if we connect to a party
  (add `KronosPartyManager.OnConnectedToPartyEvent` (`KronosPartyManager.Get`) (delegate `OnConnectedToParty_Event`))
  ;[0 0 0] Cancel matchmaking if we disconnect from the party
  (add `KronosPartyManager.OnDisconnectedFromPartyEvent` (`KronosPartyManager.Get`) (delegate `OnDisconnectedFromParty_Event`)))

(event `OnConnectedToParty_Event`
  ;[0 0 0] Cancel matchmaking if we connect to a party
  (if (`KronosStatics.IsMatchmaking`)
    (`CancelKronosMatchmakingProxy.CancelKronosMatchmaking`)))

(event `OnDisconnectedFromParty_Event`
  ;[0 0 0] Cancel matchmaking if we disconnect from the party
  (if (`KronosStatics.IsMatchmaking`)
    (`CancelKronosMatchmakingProxy.CancelKronosMatchmaking`)))

(fn `UserConstructionScript`)